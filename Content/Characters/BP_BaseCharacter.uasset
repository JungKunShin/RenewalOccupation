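; BP_BaseCharacter is a character Blueprint that walks forward automatically and halts when it detects objects ahead.
; Each Tick it adds forward movement input, then runs a multi-sphere object trace from the CheckObject component along that component's forward vector.
; Any hit calls StopMovementImmediately on CharacterMovement, though forward input is still added every frame.
; Two helper functions supply the trace endpoints, and debug drawing is enabled.
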(event `self.ReceiveTick`
  (params (DeltaSeconds :type "Float (single-precision)"))
  ;[1 1 1] 캐릭터 움직임
  (`self.AddMovementInput` (`self.GetActorForwardVector`))
  (bind (_outhits _returnvalue) (`KismetSystemLibrary.SphereTraceMultiForObjects` :`Start` (`self.Get Start Location`) :`End` (`self.GetEndLocation`) :`Radius` 200.0 :`ObjectTypes` (`self.Object Types`) :`DrawDebugType` "ForDuration"))
  (if _returnvalue
    (`MovementComponent.StopMovementImmediately` (`self.CharacterMovement`))))

(fn `Get Start Location`
  (returns (ResultValue :type "Vector Structure"))
  (return (`SceneComponent.K2_GetComponentLocation` (`self.CheckObject`))))

(fn `GetEndLocation`
  (returns (ResultValue :type "Vector Structure"))
  (return (+ (* (`KismetMathLibrary.GetForwardVector` (`SceneComponent.K2_GetComponentRotation` (`self.CheckObject`))) 500.0) (`self.Get Start Location`))))

(fn `UserConstructionScript`)