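; BP_Player1 is a character that walks forward on its own and plays a montage when it detects objects.
; Each Tick it calls SpawnDefaultController, adds forward movement input and runs a debug-drawn multi sphere trace for configured object types.
; On a hit it halts movement, plays the montage and jumps to its Default section, repeating every frame the hit persists.
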(event `self.ReceiveBeginPlay`)

(event `self.ReceiveTick`
  (params (DeltaSeconds :type "Float (single-precision)"))
  (bind _montage (`self.Montage`))
  (bind _returnvalue (`SkeletalMeshComponent.GetAnimInstance` (`self.Mesh`)))
  (`parent.ReceiveTick` DeltaSeconds)
  (`self.SpawnDefaultController`)
  (`self.AddMovementInput` (`self.GetActorForwardVector`))
  (bind (_outhits _returnvalue_2) (`KismetSystemLibrary.SphereTraceMultiForObjects` :`Start` (`self.Get Start Location`) :`End` (`self.GetEndLocation`) :`Radius` 200.0 :`ObjectTypes` (`self.Object Types`) :`DrawDebugType` "ForDuration"))
  (if _returnvalue_2
    (`MovementComponent.StopMovementImmediately` (`self.CharacterMovement`))
    (`AnimInstance.Montage_Play` _returnvalue _montage 1.0 "MontageLength" 0.0 true)
    (`AnimInstance.Montage_JumpToSection` _returnvalue "Default" _montage)))

(fn `UserConstructionScript`
  (`parent.UserConstructionScript`))