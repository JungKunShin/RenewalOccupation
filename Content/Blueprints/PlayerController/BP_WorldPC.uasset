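; BP_WorldPC is a player controller Blueprint that toggles the map and pause screens.
; The M and Q keys each flip a boolean to create and show WBP_Map or WBP_Pause, or remove it from the viewport.
; Opening either widget sets Game and UI input and shows the cursor, but closing restores neither.
; The pause toggle only manages the widget and does not pause the game here.
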(event `Key|M`
  (params (Key :type "Key Structure"))
  (bind _returnvalue (`GameplayStatics.GetPlayerController` 0))
  ;[1 1 1] 지도생성
  (:`Pressed`
    (if (`self.MapCheck`)
      (set `self.MapCheck` false)
      (bind _returnvalue_2 (`|CreateWidget` "/Game/UI/WBP_Map.WBP_Map_C" _returnvalue))
      (bind _output_get (set `self.MapWidget` _returnvalue_2))
      (`UserWidget.AddToViewport` _output_get 0)
      (`WidgetBlueprintLibrary.SetInputMode_GameAndUIEx` _returnvalue _output_get)
      (set `PlayerController.bShowMouseCursor` true _returnvalue)
      (else
        (set `self.MapCheck` true)
        (`Widget.RemoveFromParent` (`self.MapWidget`))))))

(event `Key|Q`
  (params (Key :type "Key Structure"))
  (bind _returnvalue (`GameplayStatics.GetPlayerController` 0))
  ;[1 1 1] Pause창 생성
  (:`Pressed`
    (if (`self.PauseCheck`)
      (set `self.PauseCheck` false)
      (bind _returnvalue_2 (`|CreateWidget` "/Game/UI/WBP_Pause.WBP_Pause_C" _returnvalue))
      (bind _output_get (set `self.PauseWidget` _returnvalue_2))
      (`UserWidget.AddToViewport` _output_get 0)
      (`WidgetBlueprintLibrary.SetInputMode_GameAndUIEx` _returnvalue _output_get)
      (set `PlayerController.bShowMouseCursor` true _returnvalue)
      (else
        (set `self.PauseCheck` true)
        (`Widget.RemoveFromParent` (`self.PauseWidget`))))))

(fn `UserConstructionScript`
  (`parent.UserConstructionScript`))